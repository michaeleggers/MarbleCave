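; BP_Crystal is a collectable actor that flies into the player and disappears when the player pawn overlaps it.
; The overlap plays a timeline whose alpha drives MoveToOtherActor, a swept, teleporting lerp from the crystal's current location toward the pawn's live position.
; The crystal destroys itself when the timeline finishes, with no score or inventory change in this Blueprint.
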(event EventBeginPlay)

(event Collision|EventActorBeginOverlap
  (params (OtherActor :type Actor%20Object%20Reference))
  (bind _returnvalue (Game|Player|GetPlayerPawn 0))
  (if (== OtherActor _returnvalue)
    (bind _smooth_lerp_alpha (Timeline|AlphaBlendTimeline Play)
      (:Update
        (CallFunction|MovetoOtherActor _returnvalue _smooth_lerp_alpha))
      (:Finished
        (Actor|DestroyActor)))))

(event EventTick
  (params (DeltaSeconds :type Float%20%28single-precision%29)))

(fn ConstructionScript)

(fn MovetoOtherActor
  (params (self2 :type Actor%20Object%20Reference) (Alpha :type Float%20%28single-precision%29))
  (Transformation|SetActorLocation (Math|Vector|Lerp(Vector) (Transformation|GetActorLocation) (Transformation|GetActorLocation self2) Alpha) true true))